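; Bomb ability component that spawns BP_Bomb actors, passing them radius multiplier, damage and lifetime before firing them.
; Activation calls the parent, then initializes and fires the spawned instance; UseBomb separately spawns and fires a bomb at the actor's transform.
; Construction and level-up set the radius multiplier from the skill data's ProjectileCountCurve, repurposed here as a radius curve, printing an error if the row is missing.
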(event EventActivateXform
  (params (SpawnTransform :type Transform))
  (|CallParentFunction SpawnTransform)
  (bind _spawnedactorinstance (Variables|Default|GetSpawnedActorInstance)
    (:then
      (bind _asbp_bomb (Utilities|Casting|CastToBP_Bomb _spawnedactorinstance))
      (Default|Initialize _asbp_bomb self (Variables|Default|GetRadiusMultiplier) (Variables|Default|GetDamage) (Variables|Default|GetDuration))
      (Default|Fire _asbp_bomb))
    (:else)))

(fn ConstructionScript
  (|CallParentFunction)
  (CallFunction|SetBombRadiusforLevel 1))

(fn UseBomb
  (bind _returnvalue (Game|SpawnActorfromClass (Variables|Default|GetBomb) (Transformation|GetActorTransform) "Undefined" 0 0))
  (Default|Initialize _returnvalue self (Variables|Default|GetRadiusMultiplier) (Variables|Default|GetDamage) (Variables|Default|GetDuration))
  (Default|Fire _returnvalue)
  (return _returnvalue))

(fn LevelUp
  (|CallParentFunction)
  (CallFunction|SetBombRadiusforLevel (Variables|Default|GetLevel)))

(fn SetBombRadiusforLevel
  (params (Level :type Integer))
  (bind _skilldata (Variables|Default|GetSkillData))
  (bind _projectilecountcurve (Variables|/Game/Data/BP_PDA_Ability.BP_PDA_Ability_C|GetProjectileCountCurve _skilldata))
  (bind _outxy (DataTable|EvaluateCurveTableRow (.curvetable _projectilecountcurve) (.rowname _projectilecountcurve) (Math|Conversions|ToFloat(Integer) Level))
    (:RowFound
      (Variables|Default|SetRadiusMultiplier _outxy))
    (:RowNotFound
      (Development|PrintString "Bomb Radius Curve Table Row Not Found" true true "(R=1.000000,G=0.133055,B=0.000000,A=1.000000)"))))