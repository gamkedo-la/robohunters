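; Enemy spawner that creates random enemy classes around the player, paced by a curve over elapsed time.
; Tick feeds the curve value into a Delay before each spawn.
; Spawn points come from a random ring around the player, meant to be off-camera, retried until one projects to navigable space, with a debug sphere on failure.
; MailboxBot catch events are relayed through the spawner's dispatcher; frustum math is unfinished and unused.
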(event Custom|OnMailboxCatch
  (Default|CallMailboxCatch))

(event EventBeginPlay
  (Variables|Default|SetTimeElapsed 0.0))

(event EventTick
  (params (DeltaSeconds :type Float%20%28single-precision%29))
  (bind _output_get (Variables|Default|SetTimeElapsed (+ DeltaSeconds (Variables|Default|GetTimeElapsed))))
  (Utilities|FlowControl|Delay (Math|Curves|GetFloatValue (Variables|Default|GetSpawnDelayCurve) _output_get))
  (CallFunction|SpawnEnemy))

(fn SpawnEnemy
  (bind (_location _found) (CallFunction|GetNavigableLocationOutsideCamera))
  (if _found
    (bind _returnvalue (Game|SpawnActorfromClass (.OutItem (Utilities|Array|Random (Variables|Default|GetEnemyClass))) (Math|Transform|MakeTransform _location "0, 0, 0" "1.000000,1.000000,1.000000") "Undefined" 0 0))
    (bind _asbp_mailbox_bot (Utilities|Casting|CastToBP_MailboxBot _returnvalue))
    (EventDispatchers|BindEventtoMailboxCatch _asbp_mailbox_bot (EventDispatchers|CreateEvent :!event Custom|OnMailboxCatch))
    (else
      (Rendering|Debug|DrawDebugSphere "0, 0, 0" 1e+02 12 "(R=0.545725,G=0.017642,B=0.088656,A=1.000000)" 2e+01))))

(fn GetRandomLocationOutsideCamera
  (bind _returnvalue (Game|GetPlayerCharacter 0))
  (bind _returnvalue_2 (Transformation|GetActorRotation _returnvalue))
  (Utilities|IsValid _returnvalue
    (:Is%20Valid
      (return (+ (Transformation|GetActorLocation _returnvalue) (* (Math|Rotator|GetRotationXVector (Math|Rotator|MakeRotator (.roll _returnvalue_2) (.pitch _returnvalue_2) (Math|Random|RandomFloatinRange 0.0 3.6e+02))) (Math|Random|RandomFloatinRange 1.1e+03 1.5e+03)))))))

(fn CalculateFrustrumPlane
  (params (origin :type Vector) (direcion :type Vector) (fov :type Float%20%28double-precision%29) (distance :type Float%20%28double-precision%29) (aspectRatio :type Float%20%28double-precision%29))
  (bind _output_get (LocalVariables|SetvecRight (Math|Vector|CrossProduct direcion "0.000000,1.000000,0.000000")))
  (bind _output_get_2 (LocalVariables|SetdirectionUp (Math|Vector|CrossProduct origin _output_get)))
  (bind _output_get_3 (LocalVariables|Setcenter (|((origin+direction)*distance) origin direcion distance)))
  (LocalVariables|SettopCenter (+ _output_get_2 _output_get_3))
  (LocalVariables|SetbottomCenter (- _output_get_2 _output_get_3))
  (bind _output_get_4 (LocalVariables|SetplaneHalfHeight (|((tan((fovRadians/2)))*distance) (Math|Trig|DegreesToRadians fov) distance)))
  (LocalVariables|SethalfWidth (* aspectRatio _output_get_4))
  (return (|({96399654-4DD2-80A3-87FD-80B8A2FC3BE8}-({E823E290-4D0D-4EC5-56DE-FDAF912D7EB1}*{7FFFB54C-410E-AAEC-82FE-54A7BED4585E}))) (|({96399654-4DD2-80A3-87FD-80B8A2FC3BE8}+({E823E290-4D0D-4EC5-56DE-FDAF912D7EB1}*{7FFFB54C-410E-AAEC-82FE-54A7BED4585E}))) (|({924CE67E-44AD-B35B-82CB-D7BE0BAA33A9}-({E823E290-4D0D-4EC5-56DE-FDAF912D7EB1}+{7FFFB54C-410E-AAEC-82FE-54A7BED4585E}))) (|({924CE67E-44AD-B35B-82CB-D7BE0BAA33A9}+({E823E290-4D0D-4EC5-56DE-FDAF912D7EB1}+{7FFFB54C-410E-AAEC-82FE-54A7BED4585E})))))

(fn CalculateFrustrum
  (params (origin :type Vector) (direction :type Vector) (fov :type Float%20%28double-precision%29) (nearDistane :type Float%20%28double-precision%29) (farDistance :type Float%20%28double-precision%29) (aspectRatio :type Float%20%28double-precision%29))
  (CallFunction|CalculateFrustrumPlane origin direction fov nearDistane aspectRatio)
  (CallFunction|CalculateFrustrumPlane origin direction fov farDistance aspectRatio))

(fn GetNavigableLocationOutsideCamera
  (Utilities|FlowControl|ForLoopwithBreak 0 30 :!label _label
    (:LoopBody
      (bind (_randomlocation _returnvalue) (Class|NavigationSystemV1|GetRandomLocationinNavigableRadius (CallFunction|GetRandomLocationOutsideCamera) 1e+02 0 0))
      (bind _output_get (LocalVariables|SetFoundPoint _returnvalue))
      (if _output_get
        (LocalVariables|SetNavigablePoint _randomlocation)
        (goto _label Break)))
    (:Completed
      (return (LocalVariables|GetNavigablePoint) (LocalVariables|GetFoundPoint)))))