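; Base ability for a top-down game that auto-fires at the cursor location on a cooldown while active.
; Tick counts down and spawns a pooled Niagara effect and sound at the instigator, yawed toward the cursor.
; The effect uses this object as particle collision callback, so each reported collision spawns a BP_HurtSphere, hit sound and hit effect facing the instigator.
; The construction script caches the BP_TopDownController from the instigator.
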(event EventTick
  (params (DeltaSeconds :type Float%20%28single-precision%29))
  (bind _output_get (Variables|Default|SetCooldown (- (Variables|Default|GetCooldown) DeltaSeconds)))
  (if (and (<= _output_get 0.0) (Variables|Default|GetIsActive))
    (CallFunction|Activate (Transformation|GetActorLocation (Game|GetInstigator)) (.Location (Default|GetLocationUnderCursor (Variables|Default|GetPlayerController))))
    (CallFunction|StartCooldown)))

(event EventParticleData
  (params (Data :type Array%20of%20Basic%20Particle%20Data%20Structures) (NiagaraSystem :type Niagara%20System%20Object%20Reference) (SimulationPositionOffset :type Vector%20%28by%20ref%29 :default "0, 0, 0"))
  (for _array_element Data
    (Utilities|FlowControl|Sequence
      (:then_0
        (Audio|PlaySoundatLocation (Variables|Default|GetHitSound) (.Position (Utilities|Struct|BreakBasicParticleData _array_element)) "0, 0, 0" 1.0 1.0 0.0 0 0 0 0))
      (:then_1
        (Game|SpawnActorfromClass "/Game/Actors/BP_HurtSphere.BP_HurtSphere_C" (Math|Transform|MakeTransform (.Position (Utilities|Struct|BreakBasicParticleData _array_element)) "0, 0, 0" "1.000000,1.000000,1.000000") "Undefined" 0 (Game|GetInstigator)))
      (:then_2
        (Niagara|SpawnSystematLocation (Variables|Default|GetHitEffect) (.Position (Utilities|Struct|BreakBasicParticleData _array_element)) (Math|Rotator|FindLookatRotation (.Position (Utilities|Struct|BreakBasicParticleData _array_element)) (Transformation|GetActorLocation (Game|GetInstigator))))))))

(event EventActivate
  (params (ActorLocation :type Vector :default "0, 0, 0") (TargetLocation :type Vector :default "0, 0, 0"))
  (bind _returnvalue (Niagara|SpawnSystematLocation (Variables|Default|GetActivationEffect) ActorLocation (Math|Rotator|MakeRotator 0.0 0.0 (.yaw (Math|Rotator|FindLookatRotation ActorLocation TargetLocation))) "1.000000,1.000000,1.000000" true true "AutoRelease"))
  (Class|NiagaraComponent|SetVariableObject _returnvalue "ParticleCollisionHandler" self)
  (Audio|PlaySoundatLocation (Variables|Default|GetActivationSound) ActorLocation "0, 0, 0" 1.0 1.0 0.0 0 0 0 0))

(fn ConstructionScript
  (bind _asbp_top_down_controller (Utilities|Casting|CastToBP_TopDownController (Game|GetInstigatorController)))
  (Variables|Default|SetPlayerController _asbp_top_down_controller))