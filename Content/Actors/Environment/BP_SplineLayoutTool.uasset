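; BP_SplineLayoutTool is a construction-script layout tool that places copies of a chosen mesh along a spline.
; It derives the step from the mesh bounding-box X size plus Spacing, then divides the spline length by that step to get the instance count.
; Each copy is an Instanced Static Mesh instance aligned to the spline, ignoring spline scale and offset up its local Z by half the mesh height.
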(event EventBeginPlay)

(event Collision|EventActorBeginOverlap
  (params (OtherActor :type Actor%20Object%20Reference)))

(event EventTick
  (params (DeltaSeconds :type Float%20%28single-precision%29)))

(fn ConstructionScript
  (Components|StaticMesh|SetStaticMesh (Variables|Default|GetInstancedStaticMesh) (Variables|Default|GetPlacedMesh))
  (Variables|Default|SetRealSpacing (CallFunction|CalculateSpacing))
  (bind _output_get (LocalVariables|SetNumInstances (CallFunction|CalculateNumInstances)))
  (for _index (range 0 _output_get)
    (Components|InstancedStaticMesh|AddInstance (Variables|Default|GetInstancedStaticMesh) (Math|Transform|ComposeTransforms (Spline|GetTransformatDistanceAlongSpline (Variables|Default|GetSpline) (* _index (Variables|Default|GetRealSpacing)) "Local" false) (Math|Transform|MakeTransform (Math|Vector|MakeVector 0.0 0.0 (CallFunction|BoundBoxHalfHeight)))) false)))

(fn CalculateNumInstances
  (return (Math|Float|Floor (/ (Spline|GetSplineLength (Variables|Default|GetSpline)) (Variables|Default|GetRealSpacing)))))

(fn CalculateSpacing
  (bind _placedmesh (Variables|Default|GetPlacedMesh))
  (bind _returnvalue (StaticMesh|GetBoundingBox _placedmesh))
  (bind (_min _max) (Utilities|Struct|BreakBox _returnvalue))
  (return (+ (.X (Math|Vector|BreakVector (- _max _min))) (Variables|Default|GetSpacing))))

(fn BoundBoxHalfHeight
  (bind _placedmesh (Variables|Default|GetPlacedMesh))
  (bind _returnvalue (StaticMesh|GetBoundingBox _placedmesh))
  (bind (_min _max) (Utilities|Struct|BreakBox _returnvalue))
  (return (/ (.Z (Math|Vector|BreakVector (- _max _min))) 2.0)))