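; BP_Vortex is a moving vortex that drags BP_EnemyBase actors toward its center.
; On BeginPlay it snaps to the surface below and attaches its effect, then drifts along local X.
; Overlaps and destroy events maintain the enemy set, which a Tick timer pulls horizontally using PullStrength and a distance curve normalized by VortexRadius.
; VortexChanged rescales the visual to the radius; a debug distance print remains in the pull.
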(event Custom|OnEnemyDestroyed
  (params (EnemyDestroyed :type Actor%20Object%20Reference))
  (CallFunction|RemoveEnemyfromVortex EnemyDestroyed))

(event Custom|CustomEvent
  (params (DestroyedActor :type Actor%20Object%20Reference))
  ;[1 1 1] Collision
  (CallFunction|OnEnemyDestroyed DestroyedActor))

(event Custom|VortexChanged
  (CallFunction|SetVortexRadius))

(event EventBeginPlay
  (CallFunction|Settle)
  (Niagara|SpawnSystemAttached "/Game/Actors/Vortex/FX_Vortex.FX_Vortex" (Variables|Default|GetVisual) "Socket" "0, 0, 0" "0, 0, 0" "SnapToTarget" false))

(event EventTick
  (params (DeltaSeconds :type Float%20%28single-precision%29))
  (Transformation|AddActorLocalOffset (Math|Vector|MakeVector (* DeltaSeconds 1e+02) 0.0 0.0) false false)
  (bind _output_get (Variables|Default|SetUpdateTime (+ DeltaSeconds (Variables|Default|GetUpdateTime))))
  (if (>= _output_get (Variables|Default|GetUpdateInterval))
    (CallFunction|EffectEnemiesinRadius)
    (Variables|Default|SetUpdateTime 0.0)))

(event Collision|EventActorBeginOverlap
  (params (OtherActor :type Actor%20Object%20Reference))
  ;[1 1 1] Collision
  (bind _asbp_enemy_base (Utilities|Casting|CastToBP_EnemyBase OtherActor))
  (Game|BindEventtoOnDestroyed _asbp_enemy_base (delegate Custom|CustomEvent))
  (CallFunction|AddEnemytoVortex _asbp_enemy_base))

(event Collision|EventActorEndOverlap
  (params (OtherActor :type Actor%20Object%20Reference))
  ;[1 1 1] Collision
  (bind _asbp_enemy_base (Utilities|Casting|CastToBP_EnemyBase OtherActor))
  (CallFunction|RemoveEnemyfromVortex _asbp_enemy_base))

(fn ConstructionScript)

(fn AddEnemytoVortex
  (params (ActorToAdd :type Actor%20Object%20Reference))
  (Utilities|Set|Add (Variables|Default|GetEnemiesInRadius) ActorToAdd))

(fn PullActorin
  (params (ActorToPullIn :type Actor%20Object%20Reference))
  (LocalVariables|SetActor ActorToPullIn)
  (bind _distance (CallFunction|FindDistance (LocalVariables|GetActor)))
  (bind _output_get (LocalVariables|SetDistance (/ _distance 1e+02)))
  (Development|PrintString (Utilities|String|ToString(Float) _output_get))
  (if (> _output_get 0.0)
    (Transformation|SetActorLocation (LocalVariables|GetActor) (- (Transformation|GetActorLocation (LocalVariables|GetActor)) (Math|Vector|MakeVector (.X (Math|Vector|BreakVector (* (- (Transformation|GetActorLocation (LocalVariables|GetActor)) (Transformation|GetActorLocation)) (* (Variables|Default|GetPullStrength) (- 1.0 (Math|Curves|GetFloatValue (Variables|Default|GetCurve) (/ (LocalVariables|GetDistance) (Variables|Default|GetVortexRadius)))))))) (.Y (Math|Vector|BreakVector (* (- (Transformation|GetActorLocation (LocalVariables|GetActor)) (Transformation|GetActorLocation)) (* (Variables|Default|GetPullStrength) (- 1.0 (Math|Curves|GetFloatValue (Variables|Default|GetCurve) (/ (LocalVariables|GetDistance) (Variables|Default|GetVortexRadius)))))))) 0.0)) false false)))

(fn EffectEnemiesinRadius
  (if (> (Utilities|Set|Length (Variables|Default|GetEnemiesInRadius)) 0)
    (bind _result (Utilities|Set|ToArray (Variables|Default|GetEnemiesInRadius)))
    (for _array_element _result
      (CallFunction|PullActorin _array_element))))

(fn RemoveEnemyfromVortex
  (params (ActorToRemove :type Actor%20Object%20Reference))
  (Utilities|Set|Remove (Variables|Default|GetEnemiesInRadius) ActorToRemove))

(fn SetVortexRadius
  (bind _vortexradius (Variables|Default|GetVortexRadius))
  (Transformation|SetRelativeScale3D (Variables|Default|GetVisual) (* "2.000000,2.000000,1.000000" (Math|Vector|MakeVector _vortexradius _vortexradius (.Z (Class|KismetMathLibrary|BreakVector3f (Variables|/Script/Engine.SceneComponent|GetRelativeScale3D (Variables|Default|GetVisual))))))))

(fn FindDistance
  (params (Actor :type Actor%20Object%20Reference))
  (bind _returnvalue (Transformation|GetActorLocation))
  (bind _returnvalue_2 (Transformation|GetActorLocation Actor))
  (bind (_x _y) (Math|Vector|BreakVector _returnvalue))
  (bind (_x_2 _y_2) (Math|Vector|BreakVector _returnvalue_2))
  (return (Math|Vector|Distance(Vector) (Math|Vector|MakeVector _x_2 _y_2 0.0) (Math|Vector|MakeVector _x _y 0.0))))

(fn Settle
  (bind _returnvalue (Transformation|GetActorLocation))
  (bind (_outhit _returnvalue_2) (Collision|LineTraceByChannel _returnvalue (+ _returnvalue (* (Math|Vector|NegateVector (Transformation|GetActorUpVector)) 1e+03)) "TraceTypeQuery1" false 0 "None"))
  (if _returnvalue_2
    (Transformation|SetActorLocation (.Location (Collision|BreakHitResult _outhit)) true false)))