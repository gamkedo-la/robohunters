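; Turret actor that tracks nearby enemies and switches on all its ability types at BeginPlay, with the barrel as ability origin.
; Each tick it turns the barrel toward its target while within the detection sphere's radius.
; Without a valid in-range target, it takes the first BP_EnemyBase pawn from a sphere overlap.
; After its lifetime delay it only prints a destroy message, as DestroyActor is disabled.
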(event EventBeginPlay
  (bind _abilitycomponent (Variables|Default|GetAbilityComponent))
  (for (_ _array_index) (Variables|/Game/Components/AbilityComponent.AbilityComponent_C|GetAbilityTypes _abilitycomponent)
    (Default|OnAbilityStatusChange _abilitycomponent _array_index true))
  (Utilities|FlowControl|Delay (Variables|Default|GetLifetime))
  (Development|PrintString "Destroy turret")
  (Actor|DestroyActor))

(event EventTick
  (params (DeltaSeconds :type Float%20%28single-precision%29))
  (Variables|Default|GetTarget
    (:then
      (if (CallFunction|IsTargetinRange)
        (CallFunction|LookatTarget)
        (else
          (CallFunction|AcquireTarget :!label _label))))
    (:else
      (goto _label))))

(fn ConstructionScript
  (Variables|/Game/Components/AbilityComponent.AbilityComponent_C|SetOrigin (Variables|Default|GetAbilityComponent) (Variables|Default|GetSM_Turret_barrel)))

(fn LookatTarget
  (Transformation|SetRelativeRotation (Variables|Default|GetSM_Turret_barrel) (Math|Rotator|FindLookatRotation (Transformation|GetActorLocation) (Transformation|GetActorLocation (Variables|Default|GetTarget))) false false))

(fn IsTargetinRange
  (return (< (Math|Vector|Distance(Vector) (Transformation|GetActorLocation) (Transformation|GetActorLocation (Variables|Default|GetTarget))) (Components|Sphere|GetScaledSphereRadius (Variables|Default|GetEnemyDetectionRadius)))))

(fn AcquireTarget
  (bind _enemydetectionradius (Variables|Default|GetEnemyDetectionRadius))
  (bind (_outactors _returnvalue) (Collision|SphereOverlapActors (Transformation|GetWorldLocation _enemydetectionradius) (Components|Sphere|GetScaledSphereRadius _enemydetectionradius) (Utilities|Array|MakeArray "ObjectTypeQuery3") "/Game/Actors/Enemies/BP_EnemyBase.BP_EnemyBase_C"))
  (if _returnvalue
    (bind _asbp_enemy_base (Utilities|Casting|CastToBP_EnemyBase (Utilities|Array|Get(acopy) _outactors)))
    (Variables|Default|SetTarget _asbp_enemy_base)))