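; BP_Boss is an enemy boss that rewards the player when killed.
; When its HealthComponent reports health at or below zero, it destroys itself, spawns a BP_ExperiencePickup at its transform and redundantly calls DestroyActor again.
; The same sequence then increments Kills on player 0's BP_TopDownCharacter.
; UpdateMoveSpeed sets the CharacterMovement max walk speed; BeginPlay, overlap and Tick are unused.
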(event OnHealthChanged(HealthComponent)
  (params (Health :type Float%20%28double-precision%29) (MaxHealth :type Float%20%28double-precision%29))
  (if (<= Health 0.0)
    (Utilities|FlowControl|Sequence
      (:then_0
        ;[1 1 1] Die and spawn experience pickup
        (Actor|DestroyActor)
        (Game|SpawnActorfromClass "/Game/Actors/BP_ExperiencePickup.BP_ExperiencePickup_C" (Transformation|GetActorTransform) "Undefined" 0 0)
        (Actor|DestroyActor self))
      (:then_1
        ;[1 1 1] Increase Player Kill Count
        (bind _asbp_top_down_character (Utilities|Casting|CastToBP_TopDownCharacter (Game|GetPlayerCharacter 0)))
        (Math|Integer|IncrementInt (Variables|/Game/TopDown/Blueprints/BP_TopDownCharacter.BP_TopDownCharacter_C|GetKills _asbp_top_down_character))))))

(event EventBeginPlay)

(event Collision|EventActorBeginOverlap
  (params (OtherActor :type Actor%20Object%20Reference)))

(event EventTick
  (params (DeltaSeconds :type Float%20%28single-precision%29)))

(fn ConstructionScript)

(fn UpdateMoveSpeed
  (params (Speed :type Float%20%28double-precision%29))
  (Variables|/Script/Engine.CharacterMovementComponent|SetMaxWalkSpeed (Variables|Character|GetCharacterMovement) Speed))