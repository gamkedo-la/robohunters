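; Base enemy for a top-down game that chases and attacks the player.
; Each tick it faces the player, issues AI move requests until one fails, and when CanbeAttacked is set damages the player within range, switching its range-aura material.
; Incoming damage feeds a Health component and the player's damage total.
; At zero health it destroys itself, spawns experience and possibly health pickups, and increments the player's kill count.
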(event OnHealthChanged(Health)
  (params (Health :type Float%20%28double-precision%29) (MaxHealth :type Float%20%28double-precision%29))
  (if (<= Health 0.0)
    (Utilities|FlowControl|Sequence
      (:then_0
        ;[1 1 1] Die and spawn experience pickup
        (Actor|DestroyActor)
        (Game|SpawnActorfromClass "/Game/Actors/BP_ExperiencePickup.BP_ExperiencePickup_C" (Transformation|GetActorTransform) "Undefined" 0 0)
        (Default|CallDestroyed self))
      (:then_1
        ;[1 1 1] Chance to Spawn Health Drop
        (if (< (Variables|Default|GetHealthDropChance) (Math|Random|RandomFloat))
          (Game|SpawnActorfromClass "/Game/Actors/BP_HealthPickup.BP_HealthPickup_C" (Transformation|GetActorTransform) "Undefined" 0 0)))
      (:then_2
        ;[1 1 1] Increase Player Kill Count
        (bind _asbp_top_down_character (Utilities|Casting|CastToBP_TopDownCharacter (Game|GetPlayerCharacter 0)))
        (Math|Integer|IncrementInt (Variables|/Game/TopDown/Blueprints/BP_TopDownCharacter.BP_TopDownCharacter_C|GetKills _asbp_top_down_character))))))

(event EventBeginPlay
  (Variables|Default|SetHasPath false))

(event Game|Damage|EventAnyDamage
  (params (Damage :type Float%20%28single-precision%29) (DamageType :type Damage%20Type%20Object%20Reference) (InstigatedBy :type Controller%20Object%20Reference) (DamageCauser :type Actor%20Object%20Reference))
  (Utilities|FlowControl|Sequence
    (:then_0
      (Default|TakeDamage (Variables|Default|GetHealth) Damage))
    (:then_1
      ;[1 1 1] Increase player total damage dealt
      (bind _asbp_top_down_character (Utilities|Casting|CastToBP_TopDownCharacter (Game|GetPlayerCharacter 0)))
      (Variables|/Game/TopDown/Blueprints/BP_TopDownCharacter.BP_TopDownCharacter_C|SetDamage%20Dealt _asbp_top_down_character (Math|Float|Truncate (+ Damage (Variables|/Game/TopDown/Blueprints/BP_TopDownCharacter.BP_TopDownCharacter_C|GetDamage%20Dealt _asbp_top_down_character)))))))

(event EventTick
  (params (DeltaSeconds :type Float%20%28single-precision%29))
  (bind _returnvalue (Game|GetPlayerCharacter 0))
  (Utilities|FlowControl|Sequence
    (:then_0
      (CallFunction|OrientTowardTarget)
      (bind _result (CallFunction|ShouldSeekPlayer 2.5e+02 _returnvalue))
      (if _result
        (AI|AIMoveTo self "0, 0, 0" _returnvalue (Variables|/Script/Engine.CapsuleComponent|GetCapsuleRadius (Variables|Default|GetCapsule)) true
          (:OnSuccess
            (Variables|Default|SetHasPath false))
          (:OnFail
            (Variables|Default|SetHasPath true)))))
    (:then_1
      (CallFunction|AttackPlayer))))

(fn ConstructionScript)

(fn ShouldSeekPlayer
  (params (NearRadius :type Float%20%28double-precision%29) (Target :type Actor%20Object%20Reference))
  (return (and (not (Variables|Default|GetHasPath)) (<= NearRadius (Transformation|GetDistanceTo Target)))))

(fn OrientTowardTarget
  (Transformation|SetActorRotation (Math|Rotator|FindLookatRotation (Transformation|GetActorLocation) (Transformation|GetActorLocation (Game|GetPlayerCharacter 0)))))

(fn AttackPlayer
  (bind _returnvalue (Game|GetPlayerCharacter 0))
  (bind _enemyrangeindicator (Variables|Default|GetEnemyRangeIndicator))
  ;[1 1 1] Check if target is in range
  (bind _asbp_top_down_character (Utilities|Casting|CastToBP_TopDownCharacter _returnvalue)
    (:then
      (if (<= (Math|Vector|Distance(Vector) (Transformation|GetActorLocation _asbp_top_down_character) (Transformation|GetActorLocation self)) (Variables|Default|GetAttackRange))
        (Utilities|FlowControl|Sequence
          (:then_0
            ;[1 1 1] Apply damage to target
            (if (Variables|Default|GetCanbeAttacked)
              (bind _returnvalue_2 (Game|Damage|ApplyDamage _returnvalue (Variables|Default|GetAttackDamage) 0 0))
              (Development|PrintString (Class|KismetStringLibrary|BuildStringDouble "Damage Dealt: " "" _returnvalue_2))))
          (:then_1
            ;[1 1 1] Set Correct In Range Aura Material
            (Rendering|Material|SetMaterial _enemyrangeindicator 0 "/Game/Actors/Enemies/EnemmyAura_InRange.EnemmyAura_InRange")))
        (else
          (Rendering|Material|SetMaterial _enemyrangeindicator 0 "/Game/Actors/Enemies/EnemyAura_NotInRange.EnemyAura_NotInRange"))))
    (:CastFailed
      (Development|PrintString "CheckAttackRange failed to cast to BP_TopDownCharacter object."))))