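; BP_EnemyProjectile is a pooled projectile actor launched by setting a physics velocity on its static mesh.
; Fire positions and orients the projectile and muzzle effect, then sets velocity along the actor's forward vector.
; Tick counts lifetime while visible, and Destroy hides the actor and returns it to the pool; reuse resets the timer and relaunches it.
; Hit does nothing, as damage, impact effect and muzzle effect restart are disconnected.
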(event Custom|ReuseObject
  (CallFunction|Reuse))

(event EventBeginPlay
  (EventDispatchers|BindEventtoObjectReused (Variables|Default|GetPooledObjectComponent) (delegate Custom|ReuseObject)))

(event EventTick
  (params (DeltaSeconds :type Float%20%28single-precision%29))
  (if (not (Variables|Rendering|GetbHidden))
    (CallFunction|CheckLifeSpan DeltaSeconds)))

(event Collision|EventHit
  (params (MyComp :type Primitive%20Component%20Object%20Reference) (Other :type Actor%20Object%20Reference) (OtherComp :type Primitive%20Component%20Object%20Reference) (bSelfMoved :type Boolean) (HitLocation :type Vector :default "0, 0, 0") (HitNormal :type Vector :default "0, 0, 0") (NormalImpulse :type Vector :default "0, 0, 0") (Hit :type Hit%20Result%20Structure%20%28by%20ref%29)))

(fn ConstructionScript)

(fn SetLinearVelocity
  (Transformation|SetWorldLocation (Variables|Default|GetStaticMesh) (Variables|Default|GetFirePosition) false false)
  (Physics|SetPhysicsLinearVelocity (Variables|Default|GetStaticMesh) (* (Variables|Default|GetForce) (* (Transformation|GetActorForwardVector) (LocalVariables|GetVectorForceScale))) false "None"))

(fn CheckLifeSpan
  (params (Delta :type Float%20%28double-precision%29))
  (Variables|Default|SetTimeAlive (+ Delta (Variables|Default|GetTimeAlive)))
  (if (>= (Variables|Default|GetTimeAlive) (Variables|Default|GetMaxLifeSpan))
    (CallFunction|Destroy)))

(fn Destroy
  (Rendering|SetActorHiddenInGame true)
  (Default|ReturntoPool (Variables|Default|GetPooledObjectComponent)))

(fn Reuse
  (Variables|Default|SetTimeAlive 0.0)
  (Rendering|SetActorHiddenInGame false)
  (CallFunction|SetLinearVelocity))

(fn Fire
  (params (FireRotation :type Rotator) (FirePosition :type Vector))
  (Variables|Default|SetFireRotation FireRotation)
  (Variables|Default|SetFirePosition FirePosition)
  (Transformation|SetWorldLocation (Variables|Default|GetFX_PlasmaRifleFire) (Variables|Default|GetFirePosition) false false)
  (Transformation|SetWorldRotation (Variables|Default|GetFX_PlasmaRifleFire) (Class|KismetMathLibrary|NegateRotator (Variables|Default|GetFireRotation)) false false)
  (Transformation|SetActorRotation (Variables|Default|GetFireRotation))
  (Transformation|SetWorldRotation (Variables|Default|GetStaticMesh) (Variables|Default|GetFireRotation) false false)
  (CallFunction|SetLinearVelocity))