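; BP_DroneProjectile is a projectile actor that damages the player's top-down character.
; On overlap it ignores enemies, health pickups and experience pickups through a chain of casts.
; A hit on BP_TopDownCharacter applies Damage and destroys the projectile, while any other overlapped actor just destroys it.
; A BeginPlay delay of MaxLifeSpan destroys projectiles that are still alive when it ends.
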(event EventBeginPlay
  (Utilities|FlowControl|Delay (Variables|Default|GetMaxLifeSpan))
  (Actor|DestroyActor))

(event Collision|EventActorBeginOverlap
  (params (OtherActor :type Actor%20Object%20Reference))
  (Utilities|Casting|CastToBP_EnemyBase OtherActor
    (:CastFailed
      (Utilities|Casting|CastToBP_HealthPickup OtherActor
        (:CastFailed
          (Utilities|Casting|CastToBP_ExperiencePickup OtherActor
            (:CastFailed
              (bind _asbp_top_down_character (Utilities|Casting|CastToBP_TopDownCharacter OtherActor)
                (:then
                  (Game|Damage|ApplyDamage _asbp_top_down_character (Variables|Default|GetDamage) 0 0)
                  (Actor|DestroyActor))
                (:CastFailed
                  (Actor|DestroyActor))))))))))

(event EventTick
  (params (DeltaSeconds :type Float%20%28single-precision%29)))

(fn ConstructionScript)