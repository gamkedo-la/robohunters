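; BP_DestroyerDiscAbility is an ability actor that circles a followed actor and periodically fires bursts of projectiles.
; Each tick it sets its orbit position with sine and cosine of its lifetime, then fires whenever its Cooldown component allows.
; Shots draw BP_SimpleProjectile instances from a pool, combining angular spacing with random yaw and pitch jitter.
; Increase and decrease functions step the shot count.
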(event Custom|AllowFire
  (Variables|Default|SetCanFire true))

(event EventBeginPlay)

(event EventTick
  (params (DeltaSeconds :type Float%20%28single-precision%29))
  (CallFunction|Move (Actor|GetGameTimeSinceCreation))
  (if (Variables|/Game/Components/Cooldown.Cooldown_C|GetCanTrigger (Variables|Default|GetCooldown))
    (CallFunction|FireProjectile)))

(fn ConstructionScript)

(fn Move
  (params (DeltaTime :type Float%20%28double-precision%29))
  (LocalVariables|SetElapsedTime DeltaTime)
  (LocalVariables|SetxPosition (* (+ (Math|Trig|Sin(Radians) (* (Variables|Default|GetOrbitSpeed) (LocalVariables|GetElapsedTime))) (LocalVariables|GetxPosition)) (Variables|Default|GetOrbitRadius)))
  (LocalVariables|SetyPosition (* (+ (Math|Trig|Cos(Radians) (* (Variables|Default|GetOrbitSpeed) (LocalVariables|GetElapsedTime))) (LocalVariables|GetyPosition)) (Variables|Default|GetOrbitRadius)))
  (LocalVariables|SetzPosition 5e+01)
  (Transformation|SetActorLocation (+ (Math|Vector|MakeVector (LocalVariables|GetxPosition) (LocalVariables|GetyPosition) (LocalVariables|GetzPosition)) (Transformation|GetActorLocation (Variables|Default|GetActorToFollow))) false false))

(fn FireProjectile
  (bind _numberofshots (Variables|Default|GetNumberOfShots))
  (for _index (range 0 (- _numberofshots 1))
    (LocalVariables|SetIndex _index)
    (bind _randomspread (CallFunction|CalculateSpreadRandomness 15.0))
    (bind _returnedactor (Default|GetObject (Variables|Default|GetPoolComponent)))
    (bind _asbp_simple_projectile (Utilities|Casting|CastToBP_SimpleProjectile _returnedactor))
    (Default|Fire _asbp_simple_projectile (Math|Rotator|MakeRotator 0.0 _randomspread (+ (* (LocalVariables|GetIndex) (/ 3.6e+02 (Math|Conversions|ToFloat(Integer) _numberofshots))) (Math|Random|RandomFloatinRange 0.0 3.6e+02))) (Transformation|GetActorLocation self))
    (Default|StartCooldown (Variables|Default|GetCooldown))))

(fn IncreaseNumberOfShots
  (Variables|Default|SetNumberOfShots (+ (Variables|Default|GetNumberOfShotsIncrement) (Variables|Default|GetNumberOfShots))))

(fn DecreaseNumberOfShots
  (if (>= (- (Variables|Default|GetNumberOfShots) (Variables|Default|GetNumberOfShotsIncrement)) 0)
    (Variables|Default|SetNumberOfShots (- (Variables|Default|GetNumberOfShots) (Variables|Default|GetNumberOfShotsIncrement)))))

(fn CalculateSpreadRandomness
  (params (Range :type Float%20%28double-precision%29))
  (return (+ (Variables|Default|GetSpread) (Math|Random|RandomFloatinRange Range (* -1.0 Range)))))