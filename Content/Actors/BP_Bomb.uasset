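; Bomb actor that can be dropped or fired and explodes when its lifetime runs out, or on hit if set.
; Explode applies Chaos radial strain and culled velocity fields to fracture and scatter destructibles, then sphere-overlaps pawns, excluding the instigator, to apply damage.
; An OnExplode dispatcher passes the affected actor count and triggers Niagara, sound and force feedback.
; Initialize sets damage, lifetime and the radius multiplier that scales the blast.
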(event Custom|OnExplode_Event
  (params (AffectedActorCount :type Integer))
  (bind _aoecollider (Variables|Default|GetAoECollider))
  (bind _radiusmultiplier (Variables|Default|GetRadiusMultiplier))
  (bind _returnvalue (Transformation|GetWorldLocation _aoecollider))
  (Niagara|SpawnSystematLocation "/Game/VFX/BombExplosion.BombExplosion" _returnvalue "0, 0, 0" (Math|Conversions|ToVector(Float) _radiusmultiplier) true true "AutoRelease")
  (Audio|SpawnSoundatLocation "/Game/Audio/MS_Explode.MS_Explode" _returnvalue "0, 0, 0" 1.0 1.0 0.0 0 0)
  (ForceFeedback|SpawnForceFeedbackatLocation "/Game/TopDown/Input/FFE_Bomb.FFE_Bomb" _returnvalue "0, 0, 0" false _radiusmultiplier 0.0 "/Game/TopDown/Input/FFA_BombRumbleAttenuation.FFA_BombRumbleAttenuation"))

(event EventBeginPlay
  (EventDispatchers|BindEventtoOnExplode (delegate Custom|OnExplode_Event)))

(event Collision|EventActorBeginOverlap
  (params (OtherActor :type Actor%20Object%20Reference)))

(event EventTick
  (params (DeltaSeconds :type Float%20%28single-precision%29))
  (if (Variables|/Game/Components/Lifetime.Lifetime_C|GetLifetimeExceeded (Variables|Default|GetLifetime))
    (if (not (Variables|Default|GetHasExploded))
      (CallFunction|Explode))))

(event Collision|EventHit
  (params (MyComp :type Primitive%20Component%20Object%20Reference) (Other :type Actor%20Object%20Reference) (OtherComp :type Primitive%20Component%20Object%20Reference) (bSelfMoved :type Boolean) (HitLocation :type Vector :default "0, 0, 0") (HitNormal :type Vector :default "0, 0, 0") (NormalImpulse :type Vector :default "0, 0, 0") (Hit :type Hit%20Result%20Structure%20%28by%20ref%29))
  (if (Variables|Default|GetExplodeOnContact)
    (if (not (Variables|Default|GetHasExploded))
      (CallFunction|Explode))))

(fn ConstructionScript)

(fn Explode
  (bind _radialfalloff (Variables|Default|GetRadialFalloff))
  (bind _aoecollider (Variables|Default|GetAoECollider))
  (bind _returnvalue (Components|Sphere|GetScaledSphereRadius _aoecollider))
  (bind _returnvalue_2 (Transformation|GetWorldLocation _aoecollider))
  (bind _returnvalue_3 (Field|SetRadialFalloff _radialfalloff 5e+07 0.0 1.0 0.0 _returnvalue _returnvalue_2 "Field_FallOff_None"))
  (Class|FieldSystemComponent|ApplyPhysicsField (Variables|Default|GetFieldSystem) true "Field_ExternalClusterStrain" 0 _returnvalue_3)
  (Class|FieldSystemComponent|ApplyPhysicsField (Variables|Default|GetFieldSystem) true "Field_LinearVelocity" 0 (Field|SetCullingField (Variables|Default|GetCullingField) _returnvalue_3 (Field|SetRadialVector (Variables|Default|GetRadialVector) (Variables|Default|GetForce) (Transformation|GetWorldLocation (Variables|Default|GetAoECollider))) "Field_Culling_Outside"))
  (Class|FieldSystemComponent|ResetFieldSystem (Variables|Default|GetFieldSystem))
  (Variables|Default|SetHasExploded true)
  (bind _number_affected (CallFunction|DamageEnemies))
  (Default|CallOnExplode _number_affected))

(fn DamageEnemies
  (bind _aoecollider (Variables|Default|GetAoECollider))
  (bind _returnvalue (Transformation|GetWorldLocation _aoecollider))
  (bind _sphereradius (Variables|/Script/Engine.SphereComponent|GetSphereRadius _aoecollider))
  (Rendering|Debug|DrawDebugSphere _returnvalue _sphereradius 12 "(R=0.976471,G=0.760784,B=0.168627,A=1.000000)" 1e+01)
  (bind (_outactors _returnvalue_2) (Collision|SphereOverlapActors _returnvalue _sphereradius (LocalVariables|GetSphereCastObjectTypes) "/Script/Engine.Pawn" (Utilities|Array|MakeArray (Game|GetInstigator))))
  (if _returnvalue_2
    (for _array_element _outactors
      (Game|Damage|ApplyDamage _array_element (Variables|Default|GetDamage) 0 (Components|GetOwner)))
    (return (Utilities|Array|Length _outactors))
    (else
      (Development|PrintString "No matching actors found"))))

(fn Drop
  (bind _actortospawnfrom (Variables|Default|GetActorToSpawnFrom))
  (bind _returnvalue (Transformation|GetActorTransform _actortospawnfrom))
  (Transformation|SetWorldLocationAndRotation (Variables|Default|GetDestructibleMesh) (Math|Transform|TransformLocation _returnvalue "0.000000,0.000000,200.000000") (Math|Transform|TransformRotation _returnvalue "0, 0, 0") false false))

(fn Fire
  (bind _returnvalue (Transformation|GetActorTransform))
  (Physics|SetSimulatePhysics (Variables|Default|GetDestructibleMesh) false)
  (Transformation|SetWorldLocationAndRotation (Variables|Default|GetDestructibleMesh) (Math|Transform|TransformLocation _returnvalue "0, 0, 0") (Math|Rotator|FindRelativeLookatRotation _returnvalue (Transformation|GetActorForwardVector (Game|GetInstigator))) false false)
  (Physics|SetSimulatePhysics (Variables|Default|GetDestructibleMesh) true)
  (Class|GeometryCollectionComponent|ApplyLinearVelocity (Variables|Default|GetDestructibleMesh) 0 (* (Transformation|GetActorForwardVector) (Variables|Default|GetForce))))

(fn Initialize
  (params (ActorToSpawnFrom :type Actor%20Object%20Reference) (RadiusMultiplier :type Float%20%28double-precision%29) (Damage :type Float%20%28double-precision%29) (Lifetime :type Float%20%28double-precision%29))
  (Utilities|FlowControl|Sequence
    (:then_0
      (Variables|Default|SetActorToSpawnFrom ActorToSpawnFrom))
    (:then_1
      (bind _output_get (Variables|Default|SetRadiusMultiplier RadiusMultiplier))
      (Components|Sphere|SetSphereRadius (Variables|Default|GetAoECollider) (* 1e+02 _output_get) true))
    (:then_2
      (Variables|Default|SetDamage Damage))
    (:then_3
      (Variables|/Game/Components/Lifetime.Lifetime_C|SetMaxLifetime (Variables|Default|GetLifetime) Lifetime)
      (return self))))