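; Napalm trail actor whose spline follows a target actor and damages enemies overlapping it.
; The construction script builds a spline mesh per segment.
; Tick pins the first point to ActorToFollow, then eases each later point toward its predecessor by MovementPercent, reshaping the meshes.
; Overlap and destroy events maintain the affected-enemy set, whose Health components take damage from the Tick loop, with no effective throttling despite a Delay.
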(event Custom|OnEnemyDestroyed
  (params (EnemyDestroyed :type Actor%20Object%20Reference))
  ;[1 1 1] Collision
  (CallFunction|RemoveEnemyfromAoe EnemyDestroyed))

(event Custom|CustomEvent
  (params (DestroyedActor :type Actor%20Object%20Reference))
  ;[1 1 1] Collision
  (CallFunction|OnEnemyDestroyed DestroyedActor))

(event EventBeginPlay)

(event EventTick
  (params (DeltaSeconds :type Float%20%28single-precision%29))
  (Spline|SetLocationatSplinePoint (Variables|Default|GetSpline) 0 (Transformation|GetActorLocation (Variables|Default|GetActorToFollow)) "World" true)
  (if (Variables|Default|GetPositionsCompleted)
    (Variables|Default|SetPositionsCompleted false)
    (for _index (range 1 (- (Spline|GetNumberOfSplinePoints (Variables|Default|GetSpline)) 1))
      (CallFunction|MoveSplinePoint _index)
      (if (Variables|Default|GetEnemiesDamagedCompleted)
        (bind _completed (CallFunction|DamageEnemies))
        (Utilities|FlowControl|Delay 0.2)
        (Variables|Default|SetEnemiesDamagedCompleted _completed)))
    (Variables|Default|SetPositionsCompleted true)
    (else
      (if (Variables|Default|GetEnemiesDamagedCompleted)
        (bind _completed_2 (CallFunction|DamageEnemies))
        (Utilities|FlowControl|Delay 0.2)
        (Variables|Default|SetEnemiesDamagedCompleted _completed_2)))))

(event Collision|EventActorBeginOverlap
  (params (OtherActor :type Actor%20Object%20Reference))
  ;[1 1 1] Collision
  (bind _asbp_enemy_base (Utilities|Casting|CastToBP_EnemyBase OtherActor))
  (Game|BindEventtoOnDestroyed _asbp_enemy_base (delegate Custom|CustomEvent))
  (CallFunction|AddEnemytoAoE _asbp_enemy_base))

(event Collision|EventActorEndOverlap
  (params (OtherActor :type Actor%20Object%20Reference))
  ;[1 1 1] Collision
  (bind _asbp_enemy_base (Utilities|Casting|CastToBP_EnemyBase OtherActor))
  (CallFunction|RemoveEnemyfromAoe _asbp_enemy_base))

(fn ConstructionScript
  (bind _spline (Variables|Default|GetSpline))
  (bind _spline_2 (Variables|Default|GetSpline))
  (Utilities|Set|Clear (Variables|Default|GetSplineMeshes))
  (for _index (range 0 (- (Spline|GetNumberOfSplinePoints (Variables|Default|GetSpline)) 2))
    (bind _returnvalue (AddComponent|AddSplineMeshComponent false))
    (bind _output_get (Variables|Default|SetMesh _returnvalue))
    (SplineMesh|SetForwardAxis _output_get "X" true)
    (Transformation|AttachComponentToComponent (Variables|Default|GetMesh) (Variables|Default|GetSpline) "None" "KeepRelative" "KeepRelative" "KeepRelative" true)
    (Utilities|Set|Add (Variables|Default|GetSplineMeshes) (Variables|Default|GetMesh))
    (SplineMesh|SetStartandEnd _output_get (Spline|GetLocationatSplinePoint _spline _index "Local") (Spline|GetTangentatSplinePoint _spline _index "Local") (Spline|GetLocationatSplinePoint _spline_2 (+ _index 1) "Local") (Spline|GetTangentatSplinePoint _spline_2 (+ _index 1) "Local") true :!class /Script/Engine.SplineMeshComponent)))

(fn MoveSplinePoint
  (params (Index :type Integer))
  (bind _spline (Variables|Default|GetSpline))
  (LocalVariables|SetSplinePointIndex Index)
  (LocalVariables|SetPointLocation (Spline|GetLocationatSplinePoint _spline (LocalVariables|GetSplinePointIndex) "Local"))
  (bind _output_get (LocalVariables|SetLocationDelta (- (Spline|GetLocationatSplinePoint _spline (- (LocalVariables|GetSplinePointIndex) 1) "Local") (Spline|GetLocationatSplinePoint _spline (LocalVariables|GetSplinePointIndex) "Local"))))
  (Spline|SetLocationatSplinePoint (Variables|Default|GetSpline) (LocalVariables|GetSplinePointIndex) (+ (* _output_get (LocalVariables|GetMovementPercent)) (LocalVariables|GetPointLocation)) "Local" true)
  (bind _result (Utilities|Set|ToArray (Variables|Default|GetSplineMeshes)))
  (SplineMesh|SetStartandEnd (Utilities|Array|Get(acopy) _result (- (LocalVariables|GetSplinePointIndex) 1)) (Spline|GetLocationatSplinePoint _spline (- (LocalVariables|GetSplinePointIndex) 1) "Local") (Spline|GetTangentatSplinePoint _spline (- (LocalVariables|GetSplinePointIndex) 1) "Local") (+ (* _output_get (LocalVariables|GetMovementPercent)) (LocalVariables|GetPointLocation)) (Spline|GetTangentatSplinePoint _spline (LocalVariables|GetSplinePointIndex) "Local") true :!class /Script/Engine.SplineMeshComponent))

(fn UpdateMesh)

(fn AddEnemytoAoE
  (params (ActorToAdd :type Actor%20Object%20Reference))
  (Utilities|Set|Add (Variables|Default|GetEnemiesInEffect) ActorToAdd))

(fn RemoveEnemyfromAoe
  (params (ActorToRemove :type Actor%20Object%20Reference))
  (Utilities|Set|Remove (Variables|Default|GetEnemiesInEffect) ActorToRemove))

(fn DamageEnemies
  (bind _result (Utilities|Set|ToArray (Variables|Default|GetEnemiesInEffect)))
  (for _array_element _result
    (bind _asbp_enemy_base (Utilities|Casting|CastToBP_EnemyBase _array_element))
    (Default|TakeDamage (Variables|/Game/Actors/Enemies/BP_EnemyBase.BP_EnemyBase_C|GetHealth _asbp_enemy_base) (Variables|Default|GetDamage)))
  (return true))